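; BP_MovingTarget is an enemy target actor that travels along a path and can be damaged until killed.
; On BeginPlay it finds a BP_Path actor and plays a timeline, rate-scaled by TimeToComplete, to set its transform by distance along the spline.
; Location is sampled in world space, but rotation in local space.
; HitEnnemy subtracts damage from Health, printing the remainder or destroying the actor at zero or below.
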(event Custom|MoveTarget
  (bind _path (Variables|Default|GetPath))
  (bind _spline (Variables|/Game/Anthonin/BP_Path.BP_Path_C|GetSpline _path))
  (Components|Timeline|SetPlayRate (Variables|Default|GetMove%20Target%20T) (/ 1.0 (Variables|Default|GetTime%20to%20complete)))
  (bind _move_track (Timeline|Move%20Target%20T Play)
    (:Update
      (Transformation|SetActorTransform (Math|Transform|MakeTransform (Spline|GetLocationatDistanceAlongSpline _spline (Math|Float|Lerp 0.0 (Spline|GetSplineLength (Variables|/Game/Anthonin/BP_Path.BP_Path_C|GetSpline (Variables|Default|GetPath))) _move_track) "World") (Spline|GetRotationatDistanceAlongSpline _spline (Math|Float|Lerp 0.0 (Spline|GetSplineLength (Variables|/Game/Anthonin/BP_Path.BP_Path_C|GetSpline (Variables|Default|GetPath))) _move_track) "Local") "1.000000,1.000000,1.000000")))))

(event EventBeginPlay
  (bind _returnvalue (Actor|GetActorOfClass "/Game/Anthonin/BP_Path.BP_Path_C"))
  (Variables|Default|SetPath _returnvalue)
  (CallFunction|MoveTarget))

(event EventHitEnnemy
  (params (Damage :type Integer))
  (bind _output_get (Variables|Default|SetHealth (- (Variables|Default|GetHealth) Damage)))
  (if (<= _output_get 0)
    (Development|PrintString "Ennemy Killed")
    (Actor|DestroyActor)
    (else
      (Development|PrintString (Utilities|String|ToString(Integer) _output_get) true true "(R=1.000000,G=0.119738,B=0.000000,A=1.000000)"))))

(fn ConstructionScript)