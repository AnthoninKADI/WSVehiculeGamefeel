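; BP_Health_AC is a health component, by its name, in the HealingZone folder, holding Current and Limit values with double-typed temporary copies.
; Every tick it compares the rounded TemporaryForCurrent with Current and, on a mismatch, resets the copy to Current.
; The same sync for TemporaryForLimit is nested in that branch, so it runs only when Current is out of sync.
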(event EventTick
  (params (DeltaSeconds :type Float%20%28single-precision%29))
  (if (!= (Math|Float|Round (Variables|Public|GetTemporaryForCurrent)) (Variables|Public|GetCurrent))
    (Variables|Public|SetTemporaryForCurrent (Math|Conversions|ToFloat(Integer) (Variables|Public|GetCurrent)))
    (if (!= (Math|Float|Round (Variables|Public|GetTemporaryForLimit)) (Variables|Public|GetLimit))
      (Variables|Public|SetTemporaryForLimit (Math|Conversions|ToFloat(Integer) (Variables|Public|GetLimit))))))