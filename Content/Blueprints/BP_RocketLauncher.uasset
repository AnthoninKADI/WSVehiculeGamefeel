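; Rocket launcher actor that automatically fires a pair of BP_Missile projectiles about once per second.
; Tick counts down a TimeGap timer, then resets it and spawns missiles at the RightArrow and LeftArrow transforms, adjusting for collisions but always spawning.
; Each volley briefly unhides the PSmoke1 component for half a second as a smoke effect.
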(event EventTick
  (params (DeltaSeconds :type Float%20%28single-precision%29))
  (bind _p_smoke1 (Variables|Default|GetP_Smoke1))
  (Variables|Default|SettimeGap (- (Variables|Default|GettimeGap) DeltaSeconds))
  (if (< (Variables|Default|GettimeGap) 0.0)
    (Variables|Default|SettimeGap 1.0)
    (Game|SpawnActorfromClass "/Game/Blueprints/BP_Missile.BP_Missile_C" (Transformation|GetWorldTransform (Variables|Default|GetRightArrow)) "AdjustIfPossibleButAlwaysSpawn" "MultiplyWithRoot" 0 0)
    (Game|SpawnActorfromClass "/Game/Blueprints/BP_Missile.BP_Missile_C" (Transformation|GetWorldTransform (Variables|Default|GetLeftArrow)) "AdjustIfPossibleButAlwaysSpawn" "MultiplyWithRoot" 0 0)
    (Development|SetHiddeninGame _p_smoke1 false false)
    (Utilities|FlowControl|Delay 0.5)
    (Development|SetHiddeninGame _p_smoke1 true false)))

(fn ConstructionScript)