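; BP_LaserMT is a laser projectile that damages actors implementing BPI_EnnemyHealthInterface.
; On sphere hit, it sends HitEnnemyMessage with its damage and itself, spawning an explosion effect for such actors.
; Any hit stores the impact normal and destroys the projectile.
; A destroy handler bound at BeginPlay then spawns the NS_EnemyHit effect oriented along that stored normal, so it plays whenever the laser is destroyed.
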(event OnComponentHit(Sphere)
  (params (HitComponent :type Primitive%20Component%20Object%20Reference) (OtherActor :type Actor%20Object%20Reference) (OtherComp :type Primitive%20Component%20Object%20Reference) (NormalImpulse :type Vector :default "0, 0, 0") (Hit :type Hit%20Result%20Structure%20%28by%20ref%29))
  (bind (_bblockinghit _binitialoverlap _time _distance _location _impactpoint _normal _impactnormal _physmat _hitactor) (Collision|BreakHitResult Hit))
  (Utilities|FlowControl|Sequence
    (:then_0
      ;[1 1 1] Ennemy Hit System
      (if (Utilities|DoesObjectImplementInterface _hitactor "/Game/Blueprints/Enemies/BPI_EnnemyHealthInterface.BPI_EnnemyHealthInterface_C")
        (Class|BPIEnnemyHealthInterface|HitEnnemy(Message) _hitactor (Variables|Default|GetDamage) self)
        (Niagara|SpawnSystematLocation "/Game/VFX/EnemyHitExplosion/NS_EnemyHitExpl.NS_EnemyHitExpl" _location)))
    (:then_1
      (Variables|Default|SetNormalHit _impactnormal)
      (Actor|DestroyActor))))

(event Custom|OnDestroyed_Event
  (params (DestroyedActor :type Actor%20Object%20Reference))
  (Niagara|SpawnSystematLocation "/Game/VFX/EnemyHit/NS_EnemyHit.NS_EnemyHit" (Transformation|GetActorLocation) (Math|Conversions|RotationFromXVector (Variables|Default|GetNormalHit))))

(event EventBeginPlay
  (Game|AssignOnDestroyed (delegate Custom|OnDestroyed_Event)))

(fn ConstructionScript)