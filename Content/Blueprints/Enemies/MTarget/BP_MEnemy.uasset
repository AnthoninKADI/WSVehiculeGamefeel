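; BP_MEnemy is a moving enemy target that travels along a spline path and fires lasers at the player tank.
; A timeline, rate-scaled by TimeToComplete, drives its transform along the Path spline.
; PawnSensing caches the seen tank, then Tick turns the Base toward it and spawns BP_LaserMT from the Arrow, throttled by a ShotRate Delay.
; HitEnnemy subtracts damage from Health and destroys the actor at zero.
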(event OnSeePawn(PawnSensing)
  (params (Pawn :type Pawn%20Object%20Reference))
  (bind _arrow (Variables|Default|GetArrow))
  (bind _base (Variables|Default|GetBase))
  (bind _returnvalue (Transformation|GetWorldTransform _arrow))
  (bind _asbp_tank_character (Utilities|Casting|CastToBP_TankCharacter Pawn))
  (if (Variables|/Game/_GameManager/GM_Tank.GM_Tank_C|GetcanShoot (.AsGM%20Tank (Utilities|Casting|CastToGM_Tank (Game|GetGameMode))))
    (Utilities|IsValid _asbp_tank_character
      (:Is%20Valid
        (Transformation|SetWorldRotation _base (Math|Rotator|FindLookatRotation (Transformation|GetWorldLocation _base) (Transformation|GetWorldLocation (Variables|/Script/Engine.Character|GetMesh _asbp_tank_character))) false false)
        (Utilities|FlowControl|Delay (Variables|Default|GetShot%20Rate))
        (Game|SpawnActorfromClass "/Game/Blueprints/Enemies/MTarget/BP_LaserMT.BP_LaserMT_C" (Math|Transform|MakeTransform (.location _returnvalue) (.rotation _returnvalue) "1.000000,1.000000,1.000000") "Undefined" "MultiplyWithRoot" 0 0)))))

(event Custom|MoveTarget
  (bind _path (Variables|Default|GetPath))
  (Components|Timeline|SetPlayRate (Variables|Default|GetMove%20Target%20R) (/ 1.0 (Variables|Default|GetTime%20to%20complete)))
  (bind _move_track (Timeline|Move%20Target%20R Play)
    (:Update
      (Transformation|SetActorTransform (Math|Transform|MakeTransform (Spline|GetLocationatDistanceAlongSpline (Variables|/Game/Blueprints/Enemies/MTarget/BP_Path.BP_Path_C|GetSpline _path) (Math|Float|Lerp 0.0 (Spline|GetSplineLength (Variables|/Game/Blueprints/Enemies/MTarget/BP_Path.BP_Path_C|GetSpline (Variables|Default|GetPath))) _move_track) "World") (Spline|GetRotationatDistanceAlongSpline (Variables|/Game/Blueprints/Enemies/MTarget/BP_Path.BP_Path_C|GetSpline _path) (Math|Float|Lerp 0.0 (Spline|GetSplineLength (Variables|/Game/Blueprints/Enemies/MTarget/BP_Path.BP_Path_C|GetSpline (Variables|Default|GetPath))) _move_track) "Local") "1.000000,1.000000,1.000000")))))

(event EventBeginPlay
  (Variables|Default|SetPath (Variables|Default|GetPath))
  (CallFunction|MoveTarget))

(event EventHitEnnemy
  (params (Damage :type Integer) (Projectile :type Actor%20Object%20Reference))
  (bind _output_get (Variables|Default|SetHealth (- (Variables|Default|GetHealth) Damage)))
  (if (<= _output_get 0)
    (Development|PrintString "Ennemy Killed")
    (Actor|DestroyActor)
    (else
      (Development|PrintString (Utilities|String|ToString(Integer) _output_get) true true "(R=1.000000,G=0.119738,B=0.000000,A=1.000000)"))))

(event EventTick
  (params (DeltaSeconds :type Float%20%28single-precision%29))
  (bind _arrow (Variables|Default|GetArrow))
  (bind _base (Variables|Default|GetBase))
  (bind _returnvalue (Transformation|GetWorldTransform _arrow))
  (Utilities|IsValid (stale OnSeePawn(PawnSensing) _asbp_tank_character)
    (:Is%20Valid
      (Transformation|SetWorldRotation _base (Math|Rotator|FindLookatRotation (Transformation|GetWorldLocation _base) (Transformation|GetWorldLocation (Variables|/Script/Engine.Character|GetMesh (stale OnSeePawn(PawnSensing) _asbp_tank_character)))) false false)
      (Utilities|FlowControl|Delay (Variables|Default|GetShot%20Rate))
      (Game|SpawnActorfromClass "/Game/Blueprints/Enemies/MTarget/BP_LaserMT.BP_LaserMT_C" (Math|Transform|MakeTransform (.location _returnvalue) (.rotation _returnvalue) "1.000000,1.000000,1.000000") "Undefined" "MultiplyWithRoot" 0 0))))

(fn ConstructionScript)