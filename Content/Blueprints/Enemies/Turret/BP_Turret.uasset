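; Enemy turret that aims at the player's tank and fires BP_Laser projectiles once PawnSensing has detected it.
; While the tank reference is valid, Tick drives a gate that rotates the sphere toward the tank if the game mode's CanShoot is set.
; A Delay on that path spaces shots by ShotRate.
; HitEnnemy shows a hit marker, subtracts health and destroys the turret with explosion effects at zero.
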(event OnSeePawn(PawnSensing)
  (params (Pawn :type Pawn%20Object%20Reference))
  (bind _arrow (Variables|Default|GetArrow))
  (bind _sphere (Variables|Default|GetSphere))
  (bind _returnvalue (Transformation|GetWorldTransform _arrow))
  (Development|PrintString "Player detected")
  (bind _asbp_tank_character (Utilities|Casting|CastToBP_TankCharacter Pawn)
    (:then
      (Utilities|FlowControl|Gate true :!label _label
        (:Exit
          (if (Variables|/Game/_GameManager/GM_Tank.GM_Tank_C|GetcanShoot (.AsGM%20Tank (Utilities|Casting|CastToGM_Tank (Game|GetGameMode))))
            (Transformation|SetWorldRotation _sphere (Math|Rotator|FindLookatRotation (Transformation|GetWorldLocation _sphere) (Transformation|GetWorldLocation (Variables|/Script/Engine.Character|GetMesh _asbp_tank_character))) false false)
            (Utilities|FlowControl|Delay (Variables|Default|GetShot%20Rate))
            (Game|SpawnActorfromClass "/Game/Blueprints/Enemies/Turret/BP_Laser.BP_Laser_C" (Math|Transform|MakeTransform (.location _returnvalue) (.rotation _returnvalue) "1.000000,1.000000,1.000000") "Undefined" "MultiplyWithRoot" 0 0)))))
    (:CastFailed
      (goto _label Close))))

(event EventHitEnnemy
  (params (Damage :type Integer) (Projectile :type Actor%20Object%20Reference))
  (bind _returnvalue (Transformation|GetActorTransform))
  ;[1 0.00687 0] Health / DMG
  (bind _returnvalue_2 (UserInterface|CreateWidget "/Game/UI/Common/W_HitMarker.W_HitMarker_C"))
  (UserInterface|Viewport|AddtoViewport _returnvalue_2 0)
  (Default|EventHitmarker _returnvalue_2)
  (bind _output_get (Variables|Default|SetHealth (- (Variables|Default|GetHealth) Damage)))
  (if (<= _output_get 0)
    (Niagara|SpawnSystematLocation "/Game/VFX/Ennemy_Explosions/NS_Ennemy_Explosions.NS_Ennemy_Explosions" (.location _returnvalue) (.rotation _returnvalue))
    (Audio|PlaySoundatLocation "/Game/Sounds/A_RocketExplosion_Cue.A_RocketExplosion_Cue" (Transformation|GetActorLocation) "0, 0, 0" 1.0 1.0 0.0 0 0 0 0)
    (Actor|DestroyActor)))

(event EventTick
  (params (DeltaSeconds :type Float%20%28single-precision%29))
  (bind _arrow (Variables|Default|GetArrow))
  (bind _sphere (Variables|Default|GetSphere))
  (bind _returnvalue (Transformation|GetWorldTransform _arrow))
  (Utilities|IsValid (stale OnSeePawn(PawnSensing) _asbp_tank_character)
    (:Is%20Valid
      (Utilities|FlowControl|Sequence
        (:then_0
          (goto _label Open))
        (:then_1
          (Utilities|FlowControl|Gate true :!label _label
            (:Exit
              (if (Variables|/Game/_GameManager/GM_Tank.GM_Tank_C|GetcanShoot (.AsGM%20Tank (Utilities|Casting|CastToGM_Tank (Game|GetGameMode))))
                (Transformation|SetWorldRotation _sphere (Math|Rotator|FindLookatRotation (Transformation|GetWorldLocation _sphere) (Transformation|GetWorldLocation (Variables|/Script/Engine.Character|GetMesh (stale OnSeePawn(PawnSensing) _asbp_tank_character)))) false false)
                (Utilities|FlowControl|Delay (Variables|Default|GetShot%20Rate))
                (Game|SpawnActorfromClass "/Game/Blueprints/Enemies/Turret/BP_Laser.BP_Laser_C" (Math|Transform|MakeTransform (.location _returnvalue) (.rotation _returnvalue) "1.000000,1.000000,1.000000") "Undefined" "MultiplyWithRoot" 0 0)))))))
    (:Is%20Not%20Valid
      (goto _label Close))))

(fn ConstructionScript)