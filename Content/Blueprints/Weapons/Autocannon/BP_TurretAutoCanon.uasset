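; Twin-barrel autocannon turret for the player's tank, firing projectiles from alternating barrels with camera shake, sound and magazine reloads.
; Tick turns base yaw and cannon pitch at capped speeds toward the tank's target or camera direction, keeping muzzle flashes on the barrels.
; Shoot drains a time accumulator, allowing several shots per frame at high fire rates.
; Tick also drives reload and curve-based barrel recoil; GetReloadTime exposes ammo and reload state.
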(event EventBeginPlay
  (Variables|Default|SetPlayerCameraT (Actor|GetComponentbyClass (Game|GetPlayerCharacter 0) "/Script/Engine.CameraComponent"))
  (Variables|WeaponData|SetWeaponMag (Variables|WeaponData|GetWeaponMagazineSize))
  (CallFunction|Reload)
  (Variables|Default|SetCannonRBaseLocation (Variables|/Script/Engine.SceneComponent|GetRelativeLocation (Variables|Default|GetTurretCannonR)))
  (Variables|Default|SetCannonLBaseLocation (Variables|/Script/Engine.SceneComponent|GetRelativeLocation (Variables|Default|GetTurretCannonL))))

(event Collision|EventActorBeginOverlap
  (params (OtherActor :type Actor%20Object%20Reference)))

(event EventTick
  (params (DeltaSeconds :type Float%20%28single-precision%29))
  (Utilities|TurretRotation)
  (Variables|WeaponData|SetWeaponTime (+ (Variables|WeaponData|GetWeaponTime) (* DeltaSeconds (Variables|WeaponData|GetWeaponFireRate))))
  (Utilities|ReloadMacro)
  (Utilities|CannonBackMacro))

(fn ConstructionScript)

(fn FireBullet
  (bind _lcannonarrow (Variables|Default|GetLCannonArrow))
  (bind _lcannonarrow_2 (Variables|Default|GetLCannonArrow))
  (bind _rcannonarrow (Variables|Default|GetRCannonArrow))
  (bind _rcannonarrow_2 (Variables|Default|GetRCannonArrow))
  (bind _returnvalue (Transformation|GetWorldTransform _rcannonarrow_2))
  (bind _returnvalue_2 (Transformation|GetWorldTransform _lcannonarrow))
  (bind _returnvalue_3 (Transformation|GetWorldTransform _rcannonarrow))
  (bind _returnvalue_4 (Transformation|GetWorldTransform _lcannonarrow_2))
  (Variables|WeaponData|SetWeaponMag (- (Variables|WeaponData|GetWeaponMag) 1))
  (if (Variables|WeaponData|GetCannonShootSide)
    (bind _returnvalue_5 (Game|SpawnActorfromClass "/Game/Blueprints/Weapons/Autocannon/BP_Bullet_Main.BP_Bullet_Main_C" (Math|Transform|MakeTransform (.location _returnvalue_4) (.rotation _returnvalue_4) "1.000000,1.000000,1.000000") "Undefined" "MultiplyWithRoot" (Game|Player|GetPlayerPawn 0) 0))
    (Variables|WeaponData|SetCannonShootSide false)
    (LocalVariables|SetBullet _returnvalue_5)
    (Variables|Default|SetCannonBackLT 0.0)
    (bind _returnvalue_6 (Niagara|SpawnSystematLocation "/Game/VFX/Muzzle/NS_MuzzleFlash.NS_MuzzleFlash" (.location _returnvalue_2) (.rotation _returnvalue_2) (.scale _returnvalue_2)))
    (Utilities|Array|Add (Variables|Default|GetNiagaraLCList) _returnvalue_6)
    (else
      (bind _returnvalue_7 (Game|SpawnActorfromClass "/Game/Blueprints/Weapons/Autocannon/BP_Bullet_Main.BP_Bullet_Main_C" (Math|Transform|MakeTransform (.location _returnvalue) (.rotation _returnvalue) "1.000000,1.000000,1.000000") "Undefined" "MultiplyWithRoot" (Game|Player|GetPlayerPawn 0) 0))
      (Variables|WeaponData|SetCannonShootSide true)
      (LocalVariables|SetBullet _returnvalue_7)
      (Variables|Default|SetCannonBackRT 0.0)
      (bind _returnvalue_8 (Niagara|SpawnSystematLocation "/Game/VFX/Muzzle/NS_MuzzleFlash.NS_MuzzleFlash" (.location _returnvalue_3) (.rotation _returnvalue_3) (.scale _returnvalue_3)))
      (Utilities|Array|Add (Variables|Default|GetNiagaraRCList) _returnvalue_8)))
  (Variables|/Script/Engine.ProjectileMovementComponent|SetInitialSpeed (Variables|/Game/Blueprints/Weapons/Autocannon/BP_Bullet_Main.BP_Bullet_Main_C|GetProjVelocity (LocalVariables|GetBullet)) (Variables|BulletData|GetBulletSpeed))
  (Variables|/Script/Engine.ProjectileMovementComponent|SetMaxSpeed (Variables|/Game/Blueprints/Weapons/Autocannon/BP_Bullet_Main.BP_Bullet_Main_C|GetProjVelocity (LocalVariables|GetBullet)) (Variables|BulletData|GetBulletMaxSpeed))
  (Variables|/Script/Engine.MovementComponent|SetVelocity (Variables|/Game/Blueprints/Weapons/Autocannon/BP_Bullet_Main.BP_Bullet_Main_C|GetProjVelocity (LocalVariables|GetBullet)) (* (Math|Vector|Normalize (Variables|/Script/Engine.MovementComponent|GetVelocity (Variables|/Game/Blueprints/Weapons/Autocannon/BP_Bullet_Main.BP_Bullet_Main_C|GetProjVelocity (LocalVariables|GetBullet)))) (Variables|/Script/Engine.ProjectileMovementComponent|GetInitialSpeed (Variables|/Game/Blueprints/Weapons/Autocannon/BP_Bullet_Main.BP_Bullet_Main_C|GetProjVelocity (LocalVariables|GetBullet)))))
  (Actor|SetLifeSpan (LocalVariables|GetBullet) (Variables|BulletData|GetBulletLifetime))
  (Class|LegacyCameraShake|StartLegacyCameraShake (Game|GetPlayerCameraManager 0) "/Game/Blueprints/CameraShakes/BP_CameraShake_Shooting_Primary.BP_CameraShake_Shooting_Primary_C" 1.0 "CameraLocal" "0, 0, 0"))

(fn Shoot
  (params (ButtonPressed :type Boolean))
  (if ButtonPressed
    (Variables|WeaponData|SetWeaponTime (Math|Float|Clamp(Float) (Variables|WeaponData|GetWeaponTime))))
  (if (CallFunction|CanShoot)
    (while (>= (Variables|WeaponData|GetWeaponTime) 1.0)
      (CallFunction|FireBullet)
      (Variables|WeaponData|SetWeaponTime (- (Variables|WeaponData|GetWeaponTime) 1.0))
      (Audio|PlaySound2D "/Game/Sounds/A_AutocannonShoot.A_AutocannonShoot" 1.0 1.0 0.0 0 0))))

(fn CanShoot
  (bind _weaponmag (Variables|WeaponData|GetWeaponMag))
  (bind _returnvalue (> _weaponmag 0))
  (if _returnvalue
    _
    (else
      (CallFunction|Reload)))
  (return (and _returnvalue (not (Variables|WeaponData|GetisReloading)))))

(fn Reload
  (if (and (not (Variables|WeaponData|GetisReloading)) (!= (Variables|WeaponData|GetWeaponMag) (Variables|WeaponData|GetWeaponMagazineSize)))
    (Variables|WeaponData|SetrTime (Variables|WeaponData|GetReloadTime))
    (Variables|WeaponData|SetisReloading true)))

(fn GetReloadTime
  (bind _rtime (Variables|WeaponData|GetrTime))
  (return (Variables|WeaponData|GetisReloading) _rtime (Math|Float|Clamp(Float) (- 1.0 (/ _rtime (Variables|WeaponData|GetReloadTime)))) (Variables|WeaponData|GetWeaponMag) (Variables|WeaponData|GetWeaponMagazineSize) (Math|Float|Clamp(Float) (/ (Math|Conversions|ToFloat(Integer) (Variables|WeaponData|GetWeaponMag)) (Math|Conversions|ToFloat(Integer) (Variables|WeaponData|GetWeaponMagazineSize))))))