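; Guided missile projectile that follows the player's camera aim, with a short lifespan and an explosion effect and sound on hit.
; Each Tick traces from the follow camera, ignoring third-person characters, but both branches target the trace's far end rather than the impact point.
; Rotation interpolates toward that point, while velocity keeps its speed and takes its direction from a normalized interpolated world position, not an offset from the missile.
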(event OnComponentHit(Root)
  (params (HitComponent :type Primitive%20Component%20Object%20Reference) (OtherActor :type Actor%20Object%20Reference) (OtherComp :type Primitive%20Component%20Object%20Reference) (NormalImpulse :type Vector :default "0, 0, 0") (Hit :type Hit%20Result%20Structure%20%28by%20ref%29))
  (bind _audio (Variables|Default|GetAudio))
  (Effects|SpawnEmitteratLocation "/Game/StarterContent/Particles/P_Explosion.P_Explosion" (Transformation|GetWorldLocation HitComponent))
  (Actor|SetLifeSpan 0.0001)
  (Audio|Components|Audio|SetSound _audio "/Game/Sounds/A_RocketExplosion.A_RocketExplosion")
  (Audio|Components|Audio|Play _audio 0.0))

(event EventTick
  (params (DeltaSeconds :type Float%20%28single-precision%29))
  (bind _projectilemovement (Variables|Default|GetProjectileMovement))
  (bind _projectilemovement_2 (Variables|Default|GetProjectileMovement))
  (bind _asbp_third_person_character (Utilities|Casting|CastToBP_ThirdPersonCharacter (Game|Player|GetPlayerPawn 0)))
  (bind _outactors (Actor|GetAllActorsOfClass "/Game/ThirdPerson/Blueprints/BP_ThirdPersonCharacter.BP_ThirdPersonCharacter_C"))
  (bind (_outhit _returnvalue) (Collision|LineTraceByChannel (Transformation|GetWorldLocation (Variables|/Game/ThirdPerson/Blueprints/BP_ThirdPersonCharacter.BP_ThirdPersonCharacter_C|GetFollowCamera _asbp_third_person_character)) (+ (Transformation|GetWorldLocation (Variables|/Game/ThirdPerson/Blueprints/BP_ThirdPersonCharacter.BP_ThirdPersonCharacter_C|GetFollowCamera _asbp_third_person_character)) (* (Math|Vector|GetForwardVector (Variables|/Game/ThirdPerson/Blueprints/BP_ThirdPersonCharacter.BP_ThirdPersonCharacter_C|GetFollowCamera _asbp_third_person_character)) (Variables|Default|GetMaxDist))) "TraceTypeQuery1" false _outactors "ForOneFrame"))
  (if _returnvalue
    ;[1 1 1] oriente actor
    (Transformation|SetActorRotation (Math|Interpolation|RInterpTo (Transformation|GetActorRotation) (Math|Rotator|FindLookatRotation (Transformation|GetActorLocation) (.traceend _outhit)) (Utilities|Time|GetWorldDeltaSeconds) 0.0))
    ;[1 1 1] oriente vélocité
    (Variables|/Script/Engine.MovementComponent|SetVelocity _projectilemovement (* (Math|Vector|VectorLength (Variables|/Script/Engine.MovementComponent|GetVelocity _projectilemovement)) (Math|Vector|Normalize (Math|Interpolation|VInterpTo (Transformation|GetActorLocation) (.traceend _outhit) (Utilities|Time|GetWorldDeltaSeconds) 0.0))))
    (else
      ;[1 1 1] oriente actor
      (Transformation|SetActorRotation (Math|Interpolation|RInterpTo (Transformation|GetActorRotation) (Math|Rotator|FindLookatRotation (Transformation|GetActorLocation) (+ (Transformation|GetWorldLocation (Variables|/Game/ThirdPerson/Blueprints/BP_ThirdPersonCharacter.BP_ThirdPersonCharacter_C|GetFollowCamera _asbp_third_person_character)) (* (Math|Vector|GetForwardVector (Variables|/Game/ThirdPerson/Blueprints/BP_ThirdPersonCharacter.BP_ThirdPersonCharacter_C|GetFollowCamera _asbp_third_person_character)) (Variables|Default|GetMaxDist)))) (Utilities|Time|GetWorldDeltaSeconds) 0.0))
      ;[1 1 1] oriente vélocité
      (Variables|/Script/Engine.MovementComponent|SetVelocity _projectilemovement_2 (* (Math|Vector|VectorLength (Variables|/Script/Engine.MovementComponent|GetVelocity _projectilemovement_2)) (Math|Vector|Normalize (Math|Interpolation|VInterpTo (Transformation|GetActorLocation) (+ (Transformation|GetWorldLocation (Variables|/Game/ThirdPerson/Blueprints/BP_ThirdPersonCharacter.BP_ThirdPersonCharacter_C|GetFollowCamera _asbp_third_person_character)) (* (Math|Vector|GetForwardVector (Variables|/Game/ThirdPerson/Blueprints/BP_ThirdPersonCharacter.BP_ThirdPersonCharacter_C|GetFollowCamera _asbp_third_person_character)) (Variables|Default|GetMaxDist))) (Utilities|Time|GetWorldDeltaSeconds) 0.0)))))))

(event EventBeginPlay
  (Actor|SetLifeSpan 4.0)
  (Audio|Components|Audio|Play (Variables|Default|GetAudio) 0.0))

(fn ConstructionScript)