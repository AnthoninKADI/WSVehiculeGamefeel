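; Rocket launcher that automatically fires a four-shot volley on a repeating countdown, with no input or targeting.
; Tick decrements TimeBetweenInputs and, once it drops below zero, resets it to a hardcoded interval and starts the volley.
; Chained Delays of TimeBetweenRockets stagger spawns at four arrow components, alternating left and right, top then bottom.
; Left arrows spawn BP_Missile, while the right-side spawns show no class.
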(event EventTick
  (params (DeltaSeconds :type Float%20%28single-precision%29))
  ;[1 0.4187 0.9394] Delay Between Inputs
  (Variables|Default|SettimeBetweenInputs (- (Variables|Default|GettimeBetweenInputs) DeltaSeconds))
  (if (< (Variables|Default|GettimeBetweenInputs) 0.0)
    (Variables|Default|SettimeBetweenInputs 4.0)
    ;[0.4158 1 0.6968] Delay Between Rockets
    (Game|SpawnActorfromClass "/Game/Blueprints/Weapons/Missile/BP_Missile.BP_Missile_C" (Transformation|GetWorldTransform (Variables|Default|GetLeftArrowTop)) "AdjustIfPossibleButAlwaysSpawn" "MultiplyWithRoot" 0 0)
    (Utilities|FlowControl|Delay (Variables|Default|GettimeBetweenRockets))
    (Game|SpawnActorfromClass "/Game/Blueprints/Weapons/Missile/BP_Missile.BP_Missile_C" (Transformation|GetWorldTransform (Variables|Default|GetRightArrowTop)) "AdjustIfPossibleButAlwaysSpawn" "MultiplyWithRoot" 0 0)
    (Utilities|FlowControl|Delay (Variables|Default|GettimeBetweenRockets))
    (Game|SpawnActorfromClass "/Game/Blueprints/Weapons/Missile/BP_Missile.BP_Missile_C" (Transformation|GetWorldTransform (Variables|Default|GetLeftArrowBottom)) "AdjustIfPossibleButAlwaysSpawn" "MultiplyWithRoot" 0 0)
    (Utilities|FlowControl|Delay (Variables|Default|GettimeBetweenRockets))
    (Game|SpawnActorfromClass "/Game/Blueprints/Weapons/Missile/BP_Missile.BP_Missile_C" (Transformation|GetWorldTransform (Variables|Default|GetRightArrowBottom)) "AdjustIfPossibleButAlwaysSpawn" "MultiplyWithRoot" 0 0)
    (Utilities|FlowControl|Delay (Variables|Default|GettimeBetweenRockets))))

(fn ConstructionScript)