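; BP_Wheel is a wheel actor that spins continuously at a rate set by Speed.
; Tick combines the current rotation with a negative pitch step scaled by delta time, applied after it, so the spin is about the world Y axis.
; The construction script checks the Side enum and, for one value, sets the actor's rotation to a 180-degree yaw so the wheel faces the opposite way.
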(event EventTick
  (params (DeltaSeconds :type Float%20%28single-precision%29))
  (Transformation|SetActorRotation (Math|Rotator|CombineRotators (Transformation|GetActorRotation) (Math|Rotator|MakeRotator 0.0 (* (* DeltaSeconds (Variables|Public|GetSpeed)) -1.0) 0.0))))

(fn ConstructionScript
  (if (Utilities|Enum|Equal(Enum) (Variables|Private|GetSide) "NewEnumerator1")
    (Transformation|SetActorRotation (Math|Rotator|MakeRotator 0.0 0.0 1.8e+02))))