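; Turret actor that aims by mirroring the player's camera orientation.
; On BeginPlay it finds the third-person character and caches its follow camera.
; Each tick it sets the base's world yaw to the camera's yaw and the cannon handle's world pitch to the camera's pitch, keeping the other axes unchanged.
; It contains no firing or targeting logic.
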(event EventBeginPlay
  (bind _returnvalue (Actor|GetActorOfClass "/Game/ThirdPerson/Blueprints/BP_ThirdPersonCharacter.BP_ThirdPersonCharacter_C"))
  (Variables|Default|SetPlayerCameraT (Variables|/Game/ThirdPerson/Blueprints/BP_ThirdPersonCharacter.BP_ThirdPersonCharacter_C|GetFollowCamera _returnvalue)))

(event Collision|EventActorBeginOverlap
  (params (OtherActor :type Actor%20Object%20Reference)))

(event EventTick
  (params (DeltaSeconds :type Float%20%28single-precision%29))
  (bind _playercamerat (Variables|Default|GetPlayerCameraT))
  (bind _turretbase (Variables|Default|GetTurretBase))
  (bind _turretcannonhandle (Variables|Default|GetTurretCannonHandle))
  (bind _returnvalue (Transformation|GetWorldRotation _turretbase))
  (bind _returnvalue_2 (Transformation|GetWorldRotation _turretcannonhandle))
  (bind _returnvalue_3 (Transformation|GetWorldTransform _playercamerat))
  (bind _rotation (Math|Transform|BreakTransform _returnvalue_3))
  (Transformation|SetWorldRotation _turretbase (Math|Rotator|MakeRotator (.roll _returnvalue) (.pitch _returnvalue) (.yaw _rotation)) false false)
  (Transformation|SetWorldRotation _turretcannonhandle (Math|Rotator|MakeRotator (.roll _returnvalue_2) (.pitch _rotation) (.yaw _returnvalue_2)) false false))

(fn ConstructionScript)