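; Tank game manager that runs the start countdown and decides when the player wins or loses.
; On BeginPlay it gathers all turrets as enemies and disables player input until the start timer ends, then shows the countdown widgets.
; Tick polls player health and prunes destroyed turrets, showing the win menu when none remain.
; Zero health or a missing tank calls Lose, which creates a new menu every tick, as nothing latches it.
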(event Custom|StartTimerEnd
  (Input|EnableInput (Game|GetPlayerCharacter 0) (Game|GetPlayerController 0))
  (Widget|RemovefromParent (Variables|Default|GetStartTimeWidget))
  (bind _foundwidgets (Widget|GetAllWidgetsOfClass "/Game/UI/W_CountdownTimer.W_CountdownTimer_C" true))
  (for _array_element _foundwidgets
    (Variables|/Game/UI/W_CountdownTimer.W_CountdownTimer_C|SetCountdown _array_element 0.0)
    (Widget|SetVisibility _array_element "Visible")))

(event EventBeginPlay
  (Input|SetInputModeGameOnly (Game|GetPlayerController 0) false)
  (Utilities|EnemySetup
    (:out
      (Input|DisableInput (Game|GetPlayerCharacter 0) (Game|GetPlayerController 0))
      (Utilities|Time|SetTimerbyEvent (delegate Custom|StartTimerEnd) (Variables|Default|GetTimeStart))
      (bind _returnvalue (UserInterface|CreateWidget "/Game/UI/W_StartTimer.W_StartTimer_C"))
      (bind _output_get (Variables|Default|SetStartTimeWidget _returnvalue))
      (UserInterface|Viewport|AddtoViewport _output_get 0)
      (Default|SetTimer _output_get (Variables|Default|GetTimeStart)))))

(event EventTick
  (params (DeltaSeconds :type Float%20%28single-precision%29))
  (bind _asbp_tank_character (Utilities|Casting|CastToBP_TankCharacter (Game|GetPlayerCharacter 0))
    (:then
      (if (<= (Variables|/Game/Blueprints/HealingZone/BP_Health_AC.BP_Health_AC_C|GetCurrent (Variables|/Game/_GameManager/BP_TankCharacter.BP_TankCharacter_C|GetBP_Health_AC _asbp_tank_character)) 0)
        (CallFunction|Lose :!label _label)
        (else
          (for _array_element (Variables|Default|GetEnemiesList)
            (if (not (Utilities|IsValid _array_element))
              (CallFunction|KillEnemy _array_element))))))
    (:CastFailed
      (goto _label))))

(fn ConstructionScript)

(fn KillEnemy
  (params (Enemy :type BP%20Turret%20Object%20Reference))
  (bind _returnvalue (Utilities|Array|RemoveItem (Variables|Default|GetEnemiesList) Enemy))
  (if _returnvalue
    (Variables|Default|SetEnemiesLeftToKill (- (Variables|Default|GetEnemiesLeftToKill) 1))
    (if (<= (Variables|Default|GetEnemiesLeftToKill) 0)
      (CallFunction|Win))))

(fn Win
  (bind _returnvalue (UserInterface|CreateWidget "/Game/UI/W_WinLoseMenu.W_WinLoseMenu_C"))
  (bind _output_get (Variables|Default|SetWinLoseWidget _returnvalue))
  (UserInterface|Viewport|AddtoViewport _output_get 0)
  (Default|EventWin _output_get))

(fn Lose
  (bind _returnvalue (UserInterface|CreateWidget "/Game/UI/W_WinLoseMenu.W_WinLoseMenu_C"))
  (bind _output_get (Variables|Default|SetWinLoseWidget _returnvalue))
  (UserInterface|Viewport|AddtoViewport _output_get 0)
  (Default|EventLose _output_get))