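; Twin-cannon turret that follows the player camera's yaw and pitch at limited turn speeds, firing BP_Bullet_Main projectiles from alternating left and right barrels.
; Tick accumulates a fire-rate timer that Shoot drains continuously while ammo remains and no reload runs.
; Reloading triggers at a hardcoded five rounds left, refilling the magazine after a countdown exposed through GetReloadTime.
; A float curve animates each cannon's recoil after its shot.
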(event EventBeginPlay
  (Variables|Default|SetPlayerCameraT (Actor|GetComponentbyClass (Game|GetPlayerCharacter 0) "/Script/Engine.CameraComponent"))
  (Variables|WeaponData|SetWeaponMag (Variables|WeaponData|GetWeaponMagazineSize))
  (CallFunction|Reload)
  (Variables|Default|SetCannonRBaseLocation (Variables|/Script/Engine.SceneComponent|GetRelativeLocation (Variables|Default|GetTurretCannonR)))
  (Variables|Default|SetCannonLBaseLocation (Variables|/Script/Engine.SceneComponent|GetRelativeLocation (Variables|Default|GetTurretCannonL))))

(event Collision|EventActorBeginOverlap
  (params (OtherActor :type Actor%20Object%20Reference)))

(event EventTick
  (params (DeltaSeconds :type Float%20%28single-precision%29))
  (Utilities|TurretRotation)
  (Variables|WeaponData|SetWeaponTime (+ (Variables|WeaponData|GetWeaponTime) (* DeltaSeconds (Variables|WeaponData|GetWeaponFireRate))))
  (CallFunction|Shoot false)
  (Utilities|ReloadMacro)
  (Utilities|CannonBackMacro)
  (if (== (Variables|WeaponData|GetWeaponMag) 5)
    (CallFunction|Reload)))

(fn ConstructionScript)

(fn FireBullet
  (bind _lcannonarrow (Variables|Default|GetLCannonArrow))
  (bind _rcannonarrow (Variables|Default|GetRCannonArrow))
  (bind _returnvalue (Transformation|GetWorldTransform _rcannonarrow))
  (bind _returnvalue_2 (Transformation|GetWorldTransform _lcannonarrow))
  (Variables|WeaponData|SetWeaponMag (- (Variables|WeaponData|GetWeaponMag) 1))
  (if (Variables|WeaponData|GetCannonShootSide)
    (bind _returnvalue_3 (Game|SpawnActorfromClass "/Game/Weapons/Blueprint/BP_Bullet_Main.BP_Bullet_Main_C" (Math|Transform|MakeTransform (.location _returnvalue_2) (.rotation _returnvalue_2) "1.000000,1.000000,1.000000") "Undefined" "MultiplyWithRoot" 0 0))
    (Variables|WeaponData|SetCannonShootSide false)
    (LocalVariables|SetBullet _returnvalue_3)
    (Variables|Default|SetCannonBackLT 0.0)
    (else
      (bind _returnvalue_4 (Game|SpawnActorfromClass "/Game/Weapons/Blueprint/BP_Bullet_Main.BP_Bullet_Main_C" (Math|Transform|MakeTransform (.location _returnvalue) (.rotation _returnvalue) "1.000000,1.000000,1.000000") "Undefined" "MultiplyWithRoot" 0 0))
      (Variables|WeaponData|SetCannonShootSide true)
      (LocalVariables|SetBullet _returnvalue_4)
      (Variables|Default|SetCannonBackRT 0.0)))
  (Variables|/Script/Engine.ProjectileMovementComponent|SetInitialSpeed (Variables|/Game/Weapons/Blueprint/BP_Bullet_Main.BP_Bullet_Main_C|GetProjVelocity (LocalVariables|GetBullet)) (Variables|BulletData|GetBulletSpeed))
  (Variables|/Script/Engine.ProjectileMovementComponent|SetMaxSpeed (Variables|/Game/Weapons/Blueprint/BP_Bullet_Main.BP_Bullet_Main_C|GetProjVelocity (LocalVariables|GetBullet)) (Variables|BulletData|GetBulletMaxSpeed))
  (Variables|/Game/Weapons/Blueprint/BP_Bullet_Main.BP_Bullet_Main_C|SetDamage (LocalVariables|GetBullet) (Variables|BulletData|GetBulletDamage))
  (Variables|/Script/Engine.MovementComponent|SetVelocity (Variables|/Game/Weapons/Blueprint/BP_Bullet_Main.BP_Bullet_Main_C|GetProjVelocity (LocalVariables|GetBullet)) (* (Math|Vector|Normalize (Variables|/Script/Engine.MovementComponent|GetVelocity (Variables|/Game/Weapons/Blueprint/BP_Bullet_Main.BP_Bullet_Main_C|GetProjVelocity (LocalVariables|GetBullet)))) (Variables|/Script/Engine.ProjectileMovementComponent|GetInitialSpeed (Variables|/Game/Weapons/Blueprint/BP_Bullet_Main.BP_Bullet_Main_C|GetProjVelocity (LocalVariables|GetBullet))))))

(fn Shoot
  (params (ButtonPressed :type Boolean))
  (if ButtonPressed
    (Variables|WeaponData|SetWeaponTime (Math|Float|Clamp(Float) (Variables|WeaponData|GetWeaponTime))))
  (if (CallFunction|CanShoot)
    (while (>= (Variables|WeaponData|GetWeaponTime) 1.0)
      (CallFunction|FireBullet)
      (Variables|WeaponData|SetWeaponTime (- (Variables|WeaponData|GetWeaponTime) 1.0)))))

(fn CanShoot
  (return (and (> (Variables|WeaponData|GetWeaponMag) 0) (not (Variables|WeaponData|GetisReloading)))))

(fn Reload
  (if (and (not (Variables|WeaponData|GetisReloading)) (!= (Variables|WeaponData|GetWeaponMag) (Variables|WeaponData|GetWeaponMagazineSize)))
    (Variables|WeaponData|SetrTime (Variables|WeaponData|GetReloadTime))
    (Variables|WeaponData|SetisReloading true)))

(fn GetReloadTime
  (bind _rtime (Variables|WeaponData|GetrTime))
  (return (Variables|WeaponData|GetisReloading) _rtime (Math|Float|Clamp(Float) (- 1.0 (/ _rtime (Variables|WeaponData|GetReloadTime)))) (Variables|WeaponData|GetWeaponMag) (Variables|WeaponData|GetWeaponMagazineSize) (Math|Float|Clamp(Float) (Math|Conversions|ToFloat(Integer) (/ (Variables|WeaponData|GetWeaponMag) (Variables|WeaponData|GetWeaponMagazineSize))))))