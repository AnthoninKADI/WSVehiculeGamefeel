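; BP_LaserMT is a laser actor in the MTarget enemy folder that explodes on impact and delivers damage.
; A blocking hit on its Sphere component prints a debug string, spawns P_Explosion at the impact point and destroys the actor.
; A second Sequence branch then sends Damage through HitEnnemyMessage to any hit actor implementing EnnemyHealthInterface, whether or not the hit was blocking.
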(event OnComponentHit(Sphere)
  (params (HitComponent :type Primitive%20Component%20Object%20Reference) (OtherActor :type Actor%20Object%20Reference) (OtherComp :type Primitive%20Component%20Object%20Reference) (NormalImpulse :type Vector :default "0, 0, 0") (Hit :type Hit%20Result%20Structure%20%28by%20ref%29))
  (bind (_bblockinghit _binitialoverlap _time _distance _location _impactpoint _normal _impactnormal _physmat _hitactor) (Collision|BreakHitResult Hit))
  (Utilities|FlowControl|Sequence
    (:then_0
      (if _bblockinghit
        (Development|PrintString "touch")
        (Effects|SpawnEmitteratLocation "/Game/StarterContent/Particles/P_Explosion.P_Explosion" _location)
        (Actor|DestroyActor)
        (else
          (Development|PrintString "riue"))))
    (:then_1
      ;[1 1 1] Ennemy Hit System
      (if (Utilities|DoesObjectImplementInterface _hitactor "/Game/Enemies/EnnemyHealthInterface.EnnemyHealthInterface_C")
        (Class|EnnemyHealthInterface|HitEnnemy(Message) _hitactor (Variables|Default|GetDamage))))))

(fn ConstructionScript)