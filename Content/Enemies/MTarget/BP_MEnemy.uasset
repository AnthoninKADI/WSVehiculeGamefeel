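; BP_MEnemy is a moving turret enemy that travels along a spline and shoots at the player.
; On BeginPlay it finds a BP_Path and plays a timeline, rate-scaled by TimeToComplete, to move along that spline.
; When PawnSensing sees the third-person character, it rotates its Base toward them and spawns BP_LaserMT from its Arrow after a ShotRate delay.
; A custom damage event reduces Health and destroys the actor at zero.
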(event OnSeePawn(PawnSensing)
  (params (Pawn :type Pawn%20Object%20Reference))
  (bind _returnvalue (Transformation|GetActorLocation Pawn))
  (bind _arrow (Variables|Default|GetArrow))
  (bind _base (Variables|Default|GetBase))
  (bind _returnvalue_2 (Transformation|GetWorldTransform _arrow))
  (bind (_x _y) (Class|KismetMathLibrary|BreakVector3f _returnvalue))
  (Development|PrintString "Seen Enemy")
  (Utilities|Casting|CastToBP_ThirdPersonCharacter Pawn)
  (Transformation|SetWorldRotation _base (Math|Rotator|FindLookatRotation (Transformation|GetWorldLocation _base) (Math|Vector|MakeVector _x _y 0.0)) false false)
  (Utilities|FlowControl|Delay (Variables|Default|GetShot%20Rate))
  (Game|SpawnActorfromClass "/Game/Enemies/MTarget/BP_LaserMT.BP_LaserMT_C" (Math|Transform|MakeTransform (.location _returnvalue_2) (.rotation _returnvalue_2) "1.000000,1.000000,1.000000") "Undefined" "MultiplyWithRoot" 0 0))

(event Custom|MoveTarget
  (bind _path (Variables|Default|GetPath))
  (Components|Timeline|SetPlayRate (Variables|Default|GetMove%20Target%20R) (/ 1.0 (Variables|Default|GetTime%20to%20complete)))
  (bind _move_track (Timeline|Move%20Target%20R Play)
    (:Update
      (Transformation|SetActorTransform (Math|Transform|MakeTransform (Spline|GetLocationatDistanceAlongSpline (Variables|/Game/Enemies/MTarget/BP_Path.BP_Path_C|GetSpline _path) (Math|Float|Lerp 0.0 (Spline|GetSplineLength (Variables|/Game/Enemies/MTarget/BP_Path.BP_Path_C|GetSpline (Variables|Default|GetPath))) _move_track) "World") (Spline|GetRotationatDistanceAlongSpline (Variables|/Game/Enemies/MTarget/BP_Path.BP_Path_C|GetSpline _path) (Math|Float|Lerp 0.0 (Spline|GetSplineLength (Variables|/Game/Enemies/MTarget/BP_Path.BP_Path_C|GetSpline (Variables|Default|GetPath))) _move_track) "Local") "1.000000,1.000000,1.000000")))))

(event Custom|CustomEvent
  (params (Damage :type Integer))
  (bind _output_get (Variables|Default|SetHealth (- (Variables|Default|GetHealth) Damage)))
  (if (<= _output_get 0)
    (Development|PrintString "Ennemy Killed")
    (Actor|DestroyActor)
    (else
      (Development|PrintString (Utilities|String|ToString(Integer) _output_get) true true "(R=1.000000,G=0.119738,B=0.000000,A=1.000000)"))))

(event EventBeginPlay
  (bind _returnvalue (Actor|GetActorOfClass "/Game/Enemies/MTarget/BP_Path.BP_Path_C"))
  (Variables|Default|SetPath _returnvalue)
  (CallFunction|MoveTarget))

(fn ConstructionScript)