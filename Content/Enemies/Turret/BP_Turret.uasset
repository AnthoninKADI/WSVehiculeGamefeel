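; Enemy turret that aims at the player's third-person character on sight, fires lasers and can be destroyed.
; PawnSensing turns the sphere toward the seen character's X and Y position, then a ShotRate delay paces BP_Laser spawns from the arrow's transform.
; HitEnnemy subtracts damage from health, printing the remainder or destroying the turret at zero or below.
; The AIPerception update handler is empty.
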(event OnSeePawn(PawnSensing)
  (params (Pawn :type Pawn%20Object%20Reference))
  (bind _returnvalue (Transformation|GetActorLocation Pawn))
  (bind _arrow (Variables|Default|GetArrow))
  (bind _sphere (Variables|Default|GetSphere))
  (bind _returnvalue_2 (Transformation|GetWorldTransform _arrow))
  (bind (_x _y) (Class|KismetMathLibrary|BreakVector3f _returnvalue))
  (Utilities|Casting|CastToBP_ThirdPersonCharacter Pawn)
  (Transformation|SetWorldRotation _sphere (Math|Rotator|FindLookatRotation (Transformation|GetWorldLocation _sphere) (Math|Vector|MakeVector _x _y 0.0)) false false)
  (Utilities|FlowControl|Delay (Variables|Default|GetShot%20Rate))
  (Game|SpawnActorfromClass "/Game/Enemies/Turret/BP_Laser.BP_Laser_C" (Math|Transform|MakeTransform (.location _returnvalue_2) (.rotation _returnvalue_2) "1.000000,1.000000,1.000000") "Undefined" "MultiplyWithRoot" 0 0))

(event OnPerceptionUpdated(AIPerception)
  (params (UpdatedActors :type Array%20of%20Actor%20Object%20References)))

(event EventHitEnnemy
  (params (Damage :type Integer))
  (bind _output_get (Variables|Default|SetHealth (- (Variables|Default|GetHealth) Damage)))
  (if (<= _output_get 0)
    (Development|PrintString "Ennemy Killed")
    (Actor|DestroyActor)
    (else
      (Development|PrintString (Utilities|String|ToString(Integer) _output_get) true true "(R=1.000000,G=0.119738,B=0.000000,A=1.000000)"))))

(fn ConstructionScript)